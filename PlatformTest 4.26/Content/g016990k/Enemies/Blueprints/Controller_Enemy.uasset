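; AI controller for enemies that runs the enemy behavior tree and feeds player sightings into its blackboard.
; On possession it caches the BP_Base_Enemy pawn and starts BT_Enemy.
; Perception updates on the player character set "Can See Player"; losing the player also records their current location and flags them as recently sighted.
; An Attack event forwards to the possessed enemy's own Attack.
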(event OnTargetPerceptionUpdated(AIPerception)
  (params (Actor :type Actor%20Object%20Reference) (Stimulus :type AI%20Stimulus%20Structure))
  (bind _returnvalue (AI|GetBlackboard 0))
  (Utilities|Casting|CastToThirdPersonCharacter Actor)
  (AI|Components|Blackboard|SetValueasBool _returnvalue (Utilities|Name|MakeLiteralName "Can See Player") (.bsuccessfullysensed Stimulus))
  (if (not (.bsuccessfullysensed Stimulus))
    (AI|Components|Blackboard|SetValueasVector _returnvalue (Utilities|Name|MakeLiteralName "PlayerLocation") (Transformation|GetActorLocation (Game|GetPlayerCharacter 0)))
    (AI|Components|Blackboard|SetValueasBool _returnvalue (Utilities|Name|MakeLiteralName "RecentlySighted") true)))

(event Custom|Attack
  (Default|Attack (Variables|Default|GetEnemy)))

(event EventPossess
  (params (PossessedPawn :type Pawn%20Object%20Reference))
  (bind _asbp_base_enemy (Utilities|Casting|CastToBP_Base_Enemy PossessedPawn))
  (Variables|Default|SetEnemy _asbp_base_enemy)
  (AI|RunBehaviorTree "/Game/g016990k/Enemies/Blueprints/BT_Enemy.BT_Enemy"))

(fn ConstructionScript)