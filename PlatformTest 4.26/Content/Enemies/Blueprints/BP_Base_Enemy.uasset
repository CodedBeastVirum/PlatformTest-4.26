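; Base enemy Blueprint that chases the player, takes damage and destroys itself at zero health.
; Pawn sensing turns it smoothly in yaw toward a seen ThirdPersonCharacter, then AI MoveTo closes to engagement range.
; AnyDamage feeds a clamped health update in the CharacterStats struct, then a death check.
; Combat is unfinished: the in-range timer names no function, and Attack is an uncalled print placeholder.
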(event OnSeePawn(PawnSensing)
  (params (Pawn :type Pawn%20Object%20Reference))
  (bind (_player_location _target_actor) (CallFunction|FacePlayer Pawn))
  (AI|AIMoveTo self "0, 0, 0" _target_actor (Variables|Behaviour|GetEngagement%20Range) false
    (:then
      (bind _isinrange (CallFunction|IsinRange _player_location))
      (if _isinrange
        (Utilities|Time|SetTimerbyFunctionName 0 "" 0.0)))))

(event EventBeginPlay)

(event Collision|EventActorBeginOverlap
  (params (OtherActor :type Actor%20Object%20Reference)))

(event Game|Damage|EventAnyDamage
  (params (Damage :type Float%20%28single-precision%29) (DamageType :type Damage%20Type%20Object%20Reference) (InstigatedBy :type Controller%20Object%20Reference) (DamageCauser :type Actor%20Object%20Reference))
  (CallFunction|ModifyHealth Damage false)
  (CallFunction|Death))

(fn ConstructionScript)

(fn Attack
  (Development|PrintString "Hello"))

(fn ModifyHealth
  (params (Amount :type Float%20%28single-precision%29) (Positive :type Boolean))
  (LocalVariables|SetL_Health (.health (Variables|Default|GetCharacter%20Stats)))
  (if Positive
    (LocalVariables|SetL_Health (+ (LocalVariables|GetL_Health) Amount))
    (else
      (LocalVariables|SetL_Health (- (LocalVariables|GetL_Health) Amount))))
  (bind _output_get (LocalVariables|SetL_Health (Math|Float|Clamp(Float) (LocalVariables|GetL_Health) 0.0 (.max_health (Variables|Default|GetCharacter%20Stats)))))
  (Variables|Default|SetCharacter%20Stats (Utilities|Struct|MakeEnemy_Stats _output_get 0 1e+02 2.0)))

(fn Death
  (if (<= (.health (Variables|Default|GetCharacter%20Stats)) 0.0)
    (Variables|Default|SetIsDead true)
    (Actor|DestroyActor)))

(fn FacePlayer
  (params (Target :type Pawn%20Object%20Reference))
  (bind _self self)
  (bind _returnvalue (Transformation|GetActorTransform _self))
  (bind _asthird_person_character (Utilities|Casting|CastToThirdPersonCharacter Target))
  (Transformation|SetActorRotation (Math|Rotator|MakeRotator 0.0 0.0 (.yaw (Math|Interpolation|RInterpTo (.rotation _returnvalue) (Math|Rotator|FindLookatRotation (.location _returnvalue) (Transformation|GetActorLocation _asthird_person_character)) (Utilities|Time|GetWorldDeltaSeconds) (Variables|Behaviour|GetFace%20Target%20Speed)))))
  (return (Transformation|GetActorLocation _asthird_person_character) _asthird_person_character))

(fn IsinRange
  (params (Player%20Vector :type Vector))
  (return (<= (Math|Vector|Distance(Vector) Player%20Vector (Transformation|GetActorLocation)) (Variables|Behaviour|GetEngagement%20Range))))