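; BP_EnemyDirector coordinates enemy attacks by choosing which AI in EnemyList attacks next.
; On BeginPlay it gives each enemy a random grade, scaled to the list size, and attaches a debug widget showing the enemy and its initial grade.
; A looping one-second timer makes the highest-graded enemy attack, then re-rolls that enemy's grade so turns rotate semi-randomly.
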(event Custom|Trigger%20Attack
  (bind _l_highestgradedai1 (CallFunction|FindHighestGrade))
  (Default|Attack _l_highestgradedai1)
  (Utilities|Map|Add (Variables|Default|GetEnemy%20Grading) _l_highestgradedai1 (Math|Random|RandomFloatinRange 1.0 (Math|Conversions|ToFloat(Integer) (Utilities|Array|Length (Variables|Default|GetEnemy%20List))))))

(event EventBeginPlay
  (bind _enemy_list (Variables|Default|GetEnemy%20List))
  (for _array_element _enemy_list
    (Utilities|Map|Add (Variables|Default|GetEnemy%20Grading) _array_element (Math|Random|RandomFloatinRange 1.0 (Math|Conversions|ToFloat(Integer) (Utilities|Array|Length _enemy_list))))
    (bind _returnvalue (UserInterface|CreateWidget "/Game/Enemies/Blueprints/Debug_Melee_AI.Debug_Melee_AI_C" 0 _array_element (.Value (Utilities|Map|Find (Variables|Default|GetEnemy%20Grading) _array_element))))
    (bind _returnvalue_2 (AddComponent|AddWidgetComponent _array_element false))
    (UserInterface|SetWidget _returnvalue_2 _returnvalue))
  (Utilities|Time|SetTimerbyEvent (delegate Custom|Trigger%20Attack) 1.0 true))

(fn ConstructionScript)

(fn FindHighestGrade
  (bind _enemy_grading (Variables|Default|GetEnemy%20Grading))
  (bind _keys (Utilities|Map|Keys _enemy_grading))
  (for _array_element _keys
    (if (> (.Value (Utilities|Map|Find _enemy_grading _array_element)) (LocalVariables|GetL_HighestValue))
      (LocalVariables|SetL_HighestValue (.Value (Utilities|Map|Find _enemy_grading _array_element)))
      (LocalVariables|SetL_HighestGradedAI _array_element)))
  (return (LocalVariables|GetL_HighestValue) (LocalVariables|GetL_HighestGradedAI)))