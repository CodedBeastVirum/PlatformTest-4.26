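; BP_Melee_Enemy is a melee enemy Blueprint that damages the player at close range.
; Its Attack override calls the parent, then, if CanFire is set and the player overlaps AttackRange, clears CanFire and applies the Stats damage value.
; Incoming damage reduces health through ModifyHealth, whose result decides whether Death is called.
; CanFire is not reset here, and a PlayMontage node is left unconnected.
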(event EventBeginPlay
  (|CallParentFunction) ; This node is disabled and will not be called.\nDrag off pins to build functionality.
)

(event Collision|EventActorBeginOverlap
  (params (OtherActor :type Actor%20Object%20Reference))
  (|CallParentFunction OtherActor) ; This node is disabled and will not be called.\nDrag off pins to build functionality.
)

(event EventTick
  (params (DeltaSeconds :type Float%20%28single-precision%29))
  (|CallParentFunction DeltaSeconds) ; This node is disabled and will not be called.\nDrag off pins to build functionality.
)

(event Game|Damage|EventAnyDamage
  (params (Damage :type Float%20%28single-precision%29) (DamageType :type Damage%20Type%20Object%20Reference) (InstigatedBy :type Controller%20Object%20Reference) (DamageCauser :type Actor%20Object%20Reference))
  ;[1 1 1] Damage
  (bind _isdead (CallFunction|ModifyHealth Damage false))
  (if _isdead
    (CallFunction|Death)))

(fn ConstructionScript
  (|CallParentFunction))

(fn Attack
  (bind _returnvalue (Game|GetPlayerCharacter 0))
  (|CallParentFunction)
  (if (Variables|Default|GetbCanFire)
    (if (Collision|IsOverlappingActor (Variables|Default|GetAttack%20Range) _returnvalue :!class /Script/Engine.PrimitiveComponent)
      (Variables|Default|SetbCanFire false)
      (Game|Damage|ApplyDamage _returnvalue (.damage (Variables|Default|GetStats)) 0 0))))