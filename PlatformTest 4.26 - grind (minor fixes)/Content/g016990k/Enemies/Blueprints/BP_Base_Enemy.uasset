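; BP_Base_Enemy is a base enemy actor with health, damage handling, player facing and range checking.
; A looping cooldown timer sets CanFire, while Attack is an empty stub.
; Damagedeal passes damage to ModifyHealth, which clamps health in the CharacterStats struct and triggers Death at zero, destroying the actor.
; FacePlayer smoothly interpolates yaw toward the player, and IsInRange compares a supplied position against EngagementRange.
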(event Custom|Reload
  (Variables|Default|SetbCanFire true))

(event EventBeginPlay
  (Utilities|Time|SetTimerbyEvent (delegate Custom|Reload) (.attack_cooldown (Variables|Default|GetCharacter%20Stats)) true))

(event EventDamagedeal
  (params (DamageAmount :type Float%20%28single-precision%29))
  (Development|PrintString "Hello")
  ;[1 1 1] Damage
  (bind _isdead (CallFunction|ModifyHealth DamageAmount false))
  (if _isdead
    (CallFunction|Death)))

(fn ConstructionScript)

(fn Attack
  (return))

(fn ModifyHealth
  (params (Amount :type Float%20%28single-precision%29) (Positive :type Boolean))
  (LocalVariables|SetL_Health (.health (Variables|Default|GetCharacter%20Stats)))
  (if Positive
    (LocalVariables|SetL_Health (+ (LocalVariables|GetL_Health) Amount))
    (else
      (LocalVariables|SetL_Health (- (LocalVariables|GetL_Health) Amount))))
  (bind _output_get (LocalVariables|SetL_Health (Math|Float|Clamp(Float) (LocalVariables|GetL_Health) 0.0 (.max_health (Variables|Default|GetCharacter%20Stats)))))
  (Variables|Default|SetCharacter%20Stats (Utilities|Struct|MakeEnemy_Stats _output_get 0.0 1e+02 2.0 0.0))
  (if (<= (.health (Variables|Default|GetCharacter%20Stats)) 0.0)
    (bind _output_get_2 (Variables|Default|SetbIsDead true))
    (return _output_get_2)))

(fn Death
  (Actor|DestroyActor))

(fn FacePlayer
  (bind _self self)
  (bind _returnvalue (Transformation|GetActorTransform _self))
  (Transformation|SetActorRotation (Math|Rotator|MakeRotator 0.0 0.0 (.yaw (Math|Interpolation|RInterpTo (.rotation _returnvalue) (Math|Rotator|FindLookatRotation (.location _returnvalue) (Transformation|GetActorLocation (Game|GetPlayerCharacter 0))) (Utilities|Time|GetWorldDeltaSeconds) (Variables|Behaviour|GetFace%20Target%20Speed)))))
  (return))

(fn IsinRange
  (params (Player%20Vector :type Vector))
  (return (<= (Math|Vector|Distance(Vector) Player%20Vector (Transformation|GetActorLocation)) (Variables|Behaviour|GetEngagement%20Range))))