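; Enemy wave manager that spawns successive waves of AI enemies inside a bounding box around itself, starting on BeginPlay.
; Each wave takes its size from WavePools, independently picking one of two enemy classes and one of two behavior trees per spawn.
; Spawned BP_Base_Enemy instances receive a manager reference and are counted; DeathReport decrements that count and starts the next wave at zero.
; Once waves run out, it only prints a message.
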(event Custom|Spawn_Wave
  (bind _returnvalue (Math|Random|RandomInteger 2))
  (bind _wave_pools (Variables|Default|GetWave%20Pools))
  (bind _wave_number (Variables|Default|GetWave%20Number))
  (if (>= _wave_number (Utilities|Array|Length _wave_pools))
    (Development|PrintString "They're all dead, Dave")
    (else
      (for _index (range 0 (- (Utilities|Array|Get(acopy) _wave_pools _wave_number) 1))
        (bind _returnvalue_2 (AI|SpawnAIFromClass (Utilities|Array|Get(acopy) (Variables|Default|GetEnemy%20Classes) _returnvalue) (Utilities|Array|Get(acopy) (Variables|Default|GetBehavior%20Trees) _returnvalue) (Math|Random|RandomPointinBoundingBox (Transformation|GetActorLocation) (Variables|Default|GetBoundingBoxSize)) "0, 0, 0" false 0))
        (bind _asbp_base_enemy (Utilities|Casting|CastToBP_Base_Enemy _returnvalue_2))
        (Variables|/Game/g016990k/Enemies/Blueprints/BP_Base_Enemy.BP_Base_Enemy_C|SetEnemy_Manager _asbp_base_enemy self)
        (Math|Integer|IncrementInt (Variables|Default|GetLiveEnemies)))
      (Math|Integer|IncrementInt (Variables|Default|GetWave%20Number)))))

(event Custom|Death%20Report
  (bind _liveenemies (Variables|Default|GetLiveEnemies))
  (Math|Integer|DecrementInt _liveenemies
    (:%20%20
      (if (<= _liveenemies 0)
        (CallFunction|SpawnWave)))))

(event EventBeginPlay
  (CallFunction|SpawnWave))

(event Collision|EventActorBeginOverlap
  (params (OtherActor :type Actor%20Object%20Reference)))

(fn ConstructionScript)