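; Ranged enemy Blueprint that fires projectiles and can be damaged and killed.
; Its Attack override calls the parent, then, if CanFire is set, clears that flag and always spawns a projectile at the Firepoint transform; nothing here re-arms the flag.
; The Damagedeal event subtracts health through ModifyHealth and calls Death when that returns true.
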(event EventBeginPlay
  (|CallParentFunction) ; This node is disabled and will not be called.\nDrag off pins to build functionality.
)

(event Collision|EventActorBeginOverlap
  (params (OtherActor :type Actor%20Object%20Reference))
  (|CallParentFunction OtherActor) ; This node is disabled and will not be called.\nDrag off pins to build functionality.
)

(event EventTick
  (params (DeltaSeconds :type Float%20%28single-precision%29))
  (|CallParentFunction DeltaSeconds) ; This node is disabled and will not be called.\nDrag off pins to build functionality.
)

(event EventDamagedeal
  (params (DamageAmount :type Float%20%28single-precision%29))
  ;[1 1 1] Damage
  (bind _isdead (CallFunction|ModifyHealth DamageAmount false))
  (if _isdead
    (CallFunction|Death)))

(fn ConstructionScript
  (|CallParentFunction))

(fn Attack
  (|CallParentFunction)
  (if (Variables|Default|GetbCanFire)
    (Variables|Default|SetbCanFire false)
    (Game|SpawnActorfromClass (Variables|Default|GetProjectile) (Transformation|GetWorldTransform (Variables|Default|GetFirepoint)) "AlwaysSpawn" 0 0)))